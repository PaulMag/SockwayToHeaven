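; Bunny character for a prototype that gains climb and glide abilities by touching other actors.
; Each overlap destroys the other actor, unfiltered by type, and advances one step: set CanClimb, then CanGlide, then announce the prototype's end.
; Progress rests on those two flags with printed feedback, and this graph contains no climbing or gliding movement logic.
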(event EventBeginPlay)

(event Collision|EventActorBeginOverlap
  (params (OtherActor :type Actor%20Object%20Reference))
  (if (Variables|Default|GetbCanClimb)
    (if (Variables|Default|GetbCanGlide)
      (Actor|DestroyActor OtherActor)
      (Development|PrintString "Prototype Over!")
      (else
        (Variables|Default|SetbCanGlide true)
        (Development|PrintString "Can now Glide")
        (Actor|DestroyActor OtherActor)))
    (else
      (Variables|Default|SetbCanClimb true)
      (Development|PrintString "Can now Climb")
      (Actor|DestroyActor OtherActor))))

(event EventTick
  (params (DeltaSeconds :type Float%20%28single-precision%29)))

(fn ConstructionScript)